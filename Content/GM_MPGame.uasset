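; Game mode for a local two-player game on an endlessly extendable floor of chained tiles.
; BeginPlay creates a second local player and spawns the starting tiles, each placed at the previous BP_Floor's attach point.
; ExtendFloor, not called within this Blueprint, appends a tile and destroys the oldest once the count exceeds its limit.
; Unconnected nodes hold leftover experiments with cable components on the characters.
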(event `self.ReceiveBeginPlay`
  (`GameplayStatics.CreatePlayer` 1)
  (for _ (range (`self.NumberofTiles`))
    (`self.AddFloor`)))

(fn `AddFloor`
  (bind _returnvalue (`|SpawnActorFromClass` "/Game/Blueprint/BP_Floor.BP_Floor_C" (`self.FloorAttachPoint`) "Undefined" "MultiplyWithRoot" null null))
  (bind _returnvalue_2 (`/Game/Blueprint/BP_Floor.GetAttachPoint` _returnvalue))
  (set `self.FloorAttachPoint` _returnvalue_2)
  (`KismetArrayLibrary.Array_Add` (`self.FloorTİles`) _returnvalue))

(fn `ExtendFloor`
  (bind _floorti_les (`self.FloorTİles`))
  (bind _output (`|GetArrayItem` _floorti_les))
  (`self.AddFloor`)
  (if (> (`KismetArrayLibrary.Array_Length` (`self.FloorTİles`)) (+ (`self.NumberofTiles`) 1))
    (`self.K2_DestroyActor` _output)
    (`KismetArrayLibrary.Array_RemoveItem` _floorti_les _output)))

(fn `UserConstructionScript`)